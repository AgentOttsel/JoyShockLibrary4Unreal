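; Demo character that exercises JoyShock controller input, with the left stick moving it and the right stick rotating an arrow indicator.
; On possession it builds a controller-name widget for the possessing controller and shows it on a widget component.
; Sony touchpad touches show or hide two orbs, positioned by scaled touch coordinates.
; Pressing Home sets home-light brightness to zero on every JSL4U controller assigned to that player.
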(event Input|EnhancedActionEvents|EnhancedInputActionJoyShock-RightJoystick
  (params (ActionValue :type Vector%202D%20Structure) (ElapsedSeconds :type Float%20%28double-precision%29) (TriggeredSeconds :type Float%20%28double-precision%29) (InputAction :type Input%20Action%20Object%20Reference :default "/JoyShockLibrary4Unreal/EnhancedInput/JoyShock-RightJoystick.JoyShock-RightJoystick"))
  (bind (_x _y) (Math|Vector2D|BreakVector2D ActionValue))
  (Transformation|SetWorldRotation (Variables|Default|GetJoystick%20Right%20Arrow) (Math|Rotator|MakeRotfromX (Math|Vector|MakeVector (* _x -1.0) _y 0.0)) false false))

(event Input|EnhancedActionEvents|EnhancedInputActionJoyShock-LeftJoystick
  (params (ActionValue :type Vector%202D%20Structure) (ElapsedSeconds :type Float%20%28double-precision%29) (TriggeredSeconds :type Float%20%28double-precision%29) (InputAction :type Input%20Action%20Object%20Reference :default "/JoyShockLibrary4Unreal/EnhancedInput/JoyShock-LeftJoystick.JoyShock-LeftJoystick"))
  (Pawn|Input|AddMovementInput (Math|Vector|MakeVector (.x ActionValue) (.y ActionValue) 0.0) 1.0 false))

(event Input|EnhancedActionEvents|EnhancedInputActionJoyShock-HomeButton
  (params (ActionValue :type Boolean) (ElapsedSeconds :type Float%20%28double-precision%29) (TriggeredSeconds :type Float%20%28double-precision%29) (InputAction :type Input%20Action%20Object%20Reference :default "/JoyShockLibrary4Unreal/EnhancedInput/JoyShock-HomeButton.JoyShock-HomeButton"))
  ;[0.15 0.15 0.15 0.5] Turn Off/On
  (:Started
    (for _array_element (Class|JoyShockLibrary|JSL4UGetControllersAssignedtoPlayer (stale EventPossessed NewController))
      (Class|JoyShockLibrary|JSL4USetHomeLight (.ConnectionId (Utilities|Struct|BreakJSL4UControllerInfo _array_element)) 0.0))))

(event Input|EnhancedActionEvents|EnhancedInputActionJoyShock-TouchPad1_2D
  (params (ActionValue :type Vector%202D%20Structure) (ElapsedSeconds :type Float%20%28double-precision%29) (TriggeredSeconds :type Float%20%28double-precision%29) (InputAction :type Input%20Action%20Object%20Reference :default "/JoyShockLibrary4Unreal/EnhancedInput/JoyShock-TouchPad1_2D.JoyShock-TouchPad1_2D"))
  (bind _touchpad_multiply_location (Variables|Default|GetTouchPad%20Multiply%20Location))
  (bind _returnvalue (* ActionValue _touchpad_multiply_location))
  (bind (_x _y) (Math|Vector2D|BreakVector2D _returnvalue))
  ;[0.15 0.15 0.15 0.5] Touch Pad Sony - Move Orb 1
  (Transformation|SetRelativeLocation (Variables|Default|GetSonyTouchPad1) (Math|Vector|MakeVector _x _y 0.0) false false))

(event Input|EnhancedActionEvents|EnhancedInputActionJoyShock-TouchPad2_2D
  (params (ActionValue :type Vector%202D%20Structure) (ElapsedSeconds :type Float%20%28double-precision%29) (TriggeredSeconds :type Float%20%28double-precision%29) (InputAction :type Input%20Action%20Object%20Reference :default "/JoyShockLibrary4Unreal/EnhancedInput/JoyShock-TouchPad2_2D.JoyShock-TouchPad2_2D"))
  (bind _touchpad_multiply_location (Variables|Default|GetTouchPad%20Multiply%20Location))
  (bind _returnvalue (* ActionValue _touchpad_multiply_location))
  (bind (_x _y) (Math|Vector2D|BreakVector2D _returnvalue))
  ;[0.15 0.15 0.15 0.5] TouchPad Sony - Move Orb 2
  (Transformation|SetRelativeLocation (Variables|Default|GetSonyTouchPad2) (Math|Vector|MakeVector _x _y 0.0) false false))

(event Input|EnhancedActionEvents|EnhancedInputActionJoyShock-TouchPad1_Touch
  (params (ActionValue :type Boolean) (ElapsedSeconds :type Float%20%28double-precision%29) (TriggeredSeconds :type Float%20%28double-precision%29) (InputAction :type Input%20Action%20Object%20Reference :default "/JoyShockLibrary4Unreal/EnhancedInput/JoyShock-TouchPad1_Touch.JoyShock-TouchPad1_Touch"))
  ;[0.15 0.15 0.15 0.5] Touch Pad Sony - Show Orb 1
  (:Started
    (Development|SetHiddeninGame (Variables|Default|GetSonyTouchPad1) false false))
  (:Completed
    (Development|SetHiddeninGame (Variables|Default|GetSonyTouchPad1) true false)))

(event Input|EnhancedActionEvents|EnhancedInputActionJoyShock-TouchPad2_Touch
  (params (ActionValue :type Boolean) (ElapsedSeconds :type Float%20%28double-precision%29) (TriggeredSeconds :type Float%20%28double-precision%29) (InputAction :type Input%20Action%20Object%20Reference :default "/JoyShockLibrary4Unreal/EnhancedInput/JoyShock-TouchPad2_Touch.JoyShock-TouchPad2_Touch"))
  ;[0.15 0.15 0.15 0.5] TouchPad Sony - Show Orb 2
  (:Started
    (Development|SetHiddeninGame (Variables|Default|GetSonyTouchPad2) false false))
  (:Completed
    (Development|SetHiddeninGame (Variables|Default|GetSonyTouchPad2) true false)))

(event EventPossessed
  (params (NewController :type Controller%20Object%20Reference))
  (Utilities|FlowControl|DelayUntilNextTick)
  (Class|WidgetBlueprintLibrary|SetFocustoGameViewport)
  (bind _returnvalue (UserInterface|CreateWidget "/JoyShockLibrary4Unreal/UI/WBP_ControllerName.WBP_ControllerName_C" 0 NewController))
  (UserInterface|SetWidget (Variables|Default|GetController%20Name%20Widget) _returnvalue))

(fn ConstructionScript)