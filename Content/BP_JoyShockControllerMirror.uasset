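; Actor that mirrors a physical JoyShock (JSL4U) controller in the world, with a mesh matched to its type.
; Joy-Cons refresh on pairing changes, showing grip or single mesh with body colors; Nintendo pads show player LEDs via material swaps.
; Tick applies gyro orientation as mesh rotation or, in aim mode, moves the actor by clamped yaw/pitch offsets from its starting orientation.
; Events expose gyro space and calibration controls.
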(event Custom|Reset%20Gyro%20Calibration
  (Class|JoyShockLibrary|JSL4UResetGyroCalibration (Variables|Default|GetConnection%20ID)))

(event Custom|On/Off%20Rotation%20Mode
  (params (bRotationMode :type Boolean))
  (Variables|Default|SetRotation%20Mode? bRotationMode))

(event Custom|On/Off%20Aim%20Mode
  (params (bAimMode :type Boolean))
  (bind _output_get (Variables|Default|SetAim%20Mode? bAimMode))
  (if (not _output_get)
    (Transformation|SetActorLocation (Variables|Default|GetHome%20Location) false false)))

(event Custom|Set%20Gyro%20Calibration%20Mode
  (params (Mode :type EJSL4UGyroCalibrationMode%20Enum :default "Automatic"))
  (Class|JoyShockLibrary|JSL4USetGyroCalibrationMode (Variables|Default|GetConnection%20ID) Mode))

(event Custom|Start%20Manual%20Gyro%20Calibration
  (Class|JoyShockLibrary|JSL4UStartManualGyroCalibration (Variables|Default|GetConnection%20ID)))

(event Custom|Stop%20Manual%20Gyro%20Calibration
  (Class|JoyShockLibrary|JSL4UStopManualGyroCalibration (Variables|Default|GetConnection%20ID)))

(event Custom|Gyro%20Space:%20Local
  (Class|JoyShockLibrary|JSL4USetGyroSpace (Variables|Default|GetConnection%20ID) "LocalSpace"))

(event Custom|Gyro%20Space:%20Player
  (Class|JoyShockLibrary|JSL4USetGyroSpace (Variables|Default|GetConnection%20ID) "PlayerSpace"))

(event Custom|Gyro%20Space:%20World
  (Class|JoyShockLibrary|JSL4USetGyroSpace (Variables|Default|GetConnection%20ID) "WorldSpace"))

(event EventTick
  (params (DeltaSeconds :type Float%20%28single-precision%29))
  (bind _connection_id (Variables|Default|GetConnection%20ID))
  (bind _natural_rotation (Variables|Default|GetNatural%20Rotation))
  (bind _returnvalue (Class|JoyShockLibrary|JSL4UGetMotionState _connection_id))
  (bind _returnvalue_2 (Class|KismetMathLibrary|QuatRotator (.orientation _returnvalue)))
  (bind _returnvalue_3 (Math|Rotator|Delta(Rotator) _returnvalue_2 _natural_rotation))
  (bind (_roll _pitch _yaw) (Math|Rotator|BreakRotator _returnvalue_3))
  (Utilities|FlowControl|Sequence
    (:then_0
      (if (Variables|Default|GetRotation%20Mode?)
        (Transformation|SetRelativeRotation (Variables|Default|GetSM_Controller) (Class|KismetMathLibrary|QuatRotator (.orientation (Class|JoyShockLibrary|JSL4UGetMotionState (Variables|Default|GetConnection%20ID)))) false false)
        (Utilities|FlowControl|DoOnce false :!label _label
          (:Completed
            (goto _label_2 Reset)))
        (else
          (Utilities|FlowControl|DoOnce false :!label _label_2
            (:Completed
              (Transformation|SetActorLocation self (Variables|Default|GetHome%20Location) false false)
              (goto _label Reset))))))
    (:then_1
      (if (Variables|Default|GetAim%20Mode?)
        (Transformation|SetActorLocation (+ (Math|Vector|MakeVector 0.0 (* (Math|Float|Clamp(Float) (/ _yaw (Variables|Default|GetMax%20Angle)) -1.5 1.5) (Variables|Default|GetMove%20Range)) (* (Math|Float|Clamp(Float) (/ _pitch (Variables|Default|GetMax%20Angle)) -1.0) (Variables|Default|GetMove%20Range))) "0.000000,0.000000,400.000000") false false)))))

(event EventBeginPlay
  (bind _output_get (Variables|Default|SetConnection%20ID (.ConnectionId (Utilities|Struct|BreakJSL4UControllerInfo (Variables|Controller|GetController)))))
  (Variables|Default|SetNatural%20Rotation (Class|KismetMathLibrary|QuatRotator (.orientation (Class|JoyShockLibrary|JSL4UGetMotionState _output_get))))
  (Variables|Default|SetHome%20Location (Transformation|GetActorLocation))
  (if (Class|JoyShockLibrary|JSL4UIsControllerTypeJoinable (.ControllerType (Utilities|Struct|BreakJSL4UControllerInfo (Variables|Controller|GetController))))
    (|WaitforJoyConPairingChanges
      (:then
        (CallFunction|ApplyControllerAppearance(Joycons)))
      (:OnJoined
        (CallFunction|ApplyControllerAppearance(Joycons) :!label _label))
      (:OnSeparated
        (goto _label)))
    (else
      (CallFunction|ApplyControllerAppearance(ExceptJoycons)))))

(fn ConstructionScript)

(fn ApplyControllerAppearance(ExceptJoycons)
  (switch Utilities|FlowControl|Switch|SwitchonEJSL4UControllerType (.controllertype (Variables|Controller|GetController))
    (:Undefined
      (Components|StaticMesh|SetStaticMesh (Variables|Default|GetSM_Controller) "/JoyShockLibrary4Unreal/Meshes/Xbox/Xbox.Xbox" :!label _label))
    (:XInputController
      (goto _label))
    (:DualShock4
      (Components|StaticMesh|SetStaticMesh (Variables|Default|GetSM_Controller) "/JoyShockLibrary4Unreal/Meshes/Sony/DualShock4/Dual_Shock_4.Dual_Shock_4"))
    (:DualSense
      (Components|StaticMesh|SetStaticMesh (Variables|Default|GetSM_Controller) "/JoyShockLibrary4Unreal/Meshes/Sony/DualSense/SM_Dual_Sense.SM_Dual_Sense"))
    (:ProController
      ;[0.15 0.15 0.15 0.5] Pro Controller meshes still missing
      (Components|StaticMesh|SetStaticMesh (Variables|Default|GetSM_Controller) "/JoyShockLibrary4Unreal/Meshes/Sony/DualSense/SM_Dual_Sense.SM_Dual_Sense" :!label _label_2)
      (Utilities|SetNintendoPairingLed (Variables|Controller|GetController)))
    (:ProController2
      (goto _label_2))))

(fn ApplyControllerAppearance(Joycons)
  (bind _connection_id (Variables|Default|GetConnection%20ID))
  (bind (_primarycontroller _partnercontroller _returnvalue) (Class|JoyShockLibrary|JSL4UGetJoyConPair _connection_id))
  (if (Class|JoyShockLibrary|JSL4UIsJoyConPrimary (Variables|Default|GetConnection%20ID))
    (if _returnvalue
      ;[0.15 0.15 0.15 0.5] Merged Joycon
      (Variables|Controller|SetJoy-Con%20Primary _primarycontroller)
      (Variables|Controller|SetJoy-Con%20Partner _partnercontroller)
      (CallFunction|SetStaticMesh&ResetMaterials "/JoyShockLibrary4Unreal/Meshes/Nintendo/Joy-Con(Grip)/SM_Joy-Con_Grip.SM_Joy-Con_Grip")
      (Utilities|SetJoy-ConSingleColor (Variables|Controller|GetJoy-Con%20Primary))
      (Utilities|SetJoy-ConSingleColor (Variables|Controller|GetJoy-Con%20Partner))
      (Utilities|SetNintendoPairingLed (Variables|Controller|GetController))
      (else
        ;[0.15 0.15 0.15 0.5] Sandalone Joycon
        (switch Utilities|FlowControl|Switch|SwitchonEJSL4UControllerType (.ControllerType (Utilities|Struct|BreakJSL4UControllerInfo (Variables|Controller|GetController)))
          (:JoyConLeft
            (CallFunction|SetStaticMesh&ResetMaterials "/JoyShockLibrary4Unreal/Meshes/Nintendo/Joy-Con(L)/SM_Joy-Con_L.SM_Joy-Con_L" :!label _label))
          (:JoyConRight
            (CallFunction|SetStaticMesh&ResetMaterials "/JoyShockLibrary4Unreal/Meshes/Nintendo/Joy-Con(R)/SM_Joy-Con_R.SM_Joy-Con_R" :!label _label_2))
          (:JoyCon2Left
            (goto _label))
          (:JoyCon2Right
            (goto _label_2)))
        (Utilities|SetJoy-ConSingleColor (Variables|Controller|GetController))
        (Utilities|SetNintendoPairingLed (Variables|Controller|GetController))))
    (else
      ;[0.15 0.15 0.15 0.5] Paired with another joy-con
      (Components|StaticMesh|SetStaticMesh (Variables|Default|GetSM_Controller) 0))))

(fn SetStaticMesh&ResetMaterials
  (params (NewMesh :type Static%20Mesh%20Object%20Reference))
  (Components|StaticMesh|SetStaticMesh (Variables|Default|GetSM_Controller) NewMesh)
  (for _index (range 0 (Rendering|Material|GetNumMaterials (Variables|Default|GetSM_Controller)))
    (Rendering|Material|SetMaterial (Variables|Default|GetSM_Controller) _index 0))
  (return))