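; Pawn for aiming a first-person camera with JoyShock controller gyroscope and sticks, and placing marks where it points.
; Gyro and both stick inputs scale by delta time and their own sensitivity, then feed a shared Turn event that sets control rotation with clamped, invertible pitch.
; On possession it adds the input mapping context and sets up an overlay widget.
; The right face button line-traces from the camera and spawns an aim mark at the hit.
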(event Custom|Stick%20Turn
  (params (Value :type Vector%202D%20Structure))
  (bind (_x _y) (Math|Vector2D|BreakVector2D Value))
  (bind _returnvalue (Utilities|Time|GetWorldDeltaSeconds))
  (bind _stick_speed (Variables|Default|GetStick%20Speed))
  (bind _returnvalue_2 (* _returnvalue _stick_speed))
  (CallFunction|Turn (* _y _returnvalue_2) (* (* _x _returnvalue_2) -1.0)))

(event Custom|Turn
  (params (Yaw :type Float%20%28double-precision%29) (Pitch :type Float%20%28double-precision%29))
  (bind _returnvalue (Pawn|GetControlRotation :!class /Script/Engine.Pawn))
  (bind (_roll _pitch _yaw) (Math|Rotator|BreakRotator _returnvalue))
  (Pawn|SetControlRotation (Pawn|GetController) (Math|Rotator|MakeRotator 0.0 (Math|Float|ClampAngle (+ _pitch (* Pitch (Math|Float|SelectFloat -1.0 1.0 (Variables|Default|GetInvert%20Pitch)))) -89.0 89.0) (+ _yaw Yaw))))

(event Input|EnhancedActionEvents|EnhancedInputActionJoyShock-GyroscopeRotation
  (params (ActionValue :type Vector :default "0, 0, 0") (ElapsedSeconds :type Float%20%28double-precision%29) (TriggeredSeconds :type Float%20%28double-precision%29) (InputAction :type Input%20Action%20Object%20Reference :default "/JoyShockLibrary4Unreal/EnhancedInput/JoyShock-GyroscopeRotation.JoyShock-GyroscopeRotation"))
  (bind _returnvalue (Utilities|Time|GetWorldDeltaSeconds))
  (bind _sensitivity (Variables|Default|GetSensitivity))
  (bind _returnvalue_2 (* _returnvalue _sensitivity))
  (bind _returnvalue_3 (* ActionValue _returnvalue_2))
  (bind (_x _y _z) (Math|Vector|BreakVector _returnvalue_3))
  (CallFunction|Turn _z _y))

(event Input|EnhancedActionEvents|EnhancedInputActionJoyShock-RightJoystick
  (params (ActionValue :type Vector%202D%20Structure) (ElapsedSeconds :type Float%20%28double-precision%29) (TriggeredSeconds :type Float%20%28double-precision%29) (InputAction :type Input%20Action%20Object%20Reference :default "/JoyShockLibrary4Unreal/EnhancedInput/JoyShock-RightJoystick.JoyShock-RightJoystick"))
  (CallFunction|StickTurn ActionValue))

(event Input|EnhancedActionEvents|EnhancedInputActionJoyShock-LeftJoystick
  (params (ActionValue :type Vector%202D%20Structure) (ElapsedSeconds :type Float%20%28double-precision%29) (TriggeredSeconds :type Float%20%28double-precision%29) (InputAction :type Input%20Action%20Object%20Reference :default "/JoyShockLibrary4Unreal/EnhancedInput/JoyShock-LeftJoystick.JoyShock-LeftJoystick"))
  (CallFunction|StickTurn (* ActionValue "(X=-1.000000,Y=1.000000)")))

(event Input|EnhancedActionEvents|EnhancedInputActionJoyShock-FaceButtonRight
  (params (ActionValue :type Boolean) (ElapsedSeconds :type Float%20%28double-precision%29) (TriggeredSeconds :type Float%20%28double-precision%29) (InputAction :type Input%20Action%20Object%20Reference :default "/JoyShockLibrary4Unreal/EnhancedInput/JoyShock-FaceButtonRight.JoyShock-FaceButtonRight"))
  (bind _camera (Variables|Default|GetCamera))
  (bind _returnvalue (Transformation|GetWorldLocation _camera))
  (:Started
    (bind (_outhit _returnvalue_2) (Collision|LineTraceByChannel _returnvalue (+ _returnvalue (* (Math|Vector|GetForwardVector _camera) 1e+04)) "TraceTypeQuery1" false 0 "None"))
    (if _returnvalue_2
      (Game|SpawnActorfromClass "/JoyShockLibrary4Unreal/BP_JoyShockGyroAimMark.BP_JoyShockGyroAimMark_C" (Math|Transform|MakeTransform (.Location (Collision|BreakHitResult _outhit)) "0, 0, 0" "1.000000,1.000000,1.000000") "Undefined" "MultiplyWithRoot" 0 0))))

(event EventPossessed
  (params (NewController :type Controller%20Object%20Reference))
  (bind _returnvalue (Game|GetPlayerController 0))
  (bind _asplayer_controller (Utilities|Casting|CastToPlayerController NewController))
  (Input|AddMappingContext (PlayerController|LocalPlayerSubsystems|GetEnhancedInputLocalPlayerSubsystem _asplayer_controller) "/JoyShockLibrary4Unreal/EnhancedInput/JoyShockInputMappingContext.JoyShockInputMappingContext" 0 "(bIgnoreAllPressedKeysUntilRelease=True,bForceImmediately=False,bNotifyUserSettings=False)")
  (Game|Player|SetViewTargetwithBlend _returnvalue self 0.0 "VTBlend_Linear" 0.0 false)
  (if (Utilities|IsValid (Variables|Default|GetOverlay))
    (Utilities|FlowControl|DelayUntilNextTick)
    (Class|WidgetBlueprintLibrary|SetFocustoGameViewport)
    (else
      (bind _returnvalue_2 (UserInterface|CreateWidget "/JoyShockLibrary4Unreal/UI/WBP_JoyShockGyroAimOverlay.WBP_JoyShockGyroAimOverlay_C" _returnvalue))
      (UserInterface|Viewport|AddtoViewport _returnvalue_2 0)
      (Variables|Default|SetOverlay _returnvalue_2)
      (Variables|/Script/Engine.PlayerController|SetbShowMouseCursor _returnvalue true)
      (Input|SetInputModeGameandUI _returnvalue 0 "DoNotLock" false false))))

(fn ConstructionScript)