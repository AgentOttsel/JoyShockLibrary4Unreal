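; Actor that visualizes gyro motion of controller device 0 through JoyShockLibrary (Jsl) calls.
; BeginPlay connects devices and starts continuous calibration; custom events switch gyro space, calibration, tick and the two modes.
; On Tick, rotation mode applies the motion quaternion with axes remapped to Unreal.
; Aim mode prints the flushed accumulated gyro and moves the actor along world Y and Z, without delta-time scaling.
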(event Custom|StillConnected
  (bind _returnvalue (Class|JoyShockLibrary|JslStillConnected))
  (Development|PrintString (Utilities|String|ToString(Boolean) _returnvalue) true false))

(event Custom|ConnectDevices
  (bind _returnvalue (Class|JoyShockLibrary|JslConnectDevices))
  (Development|PrintString (Utilities|String|ToString(Integer) _returnvalue) true false))

(event Custom|ToggleRotationMode
  (Variables|Default|SetbRotationMode (not (Variables|Default|GetbRotationMode))))

(event Custom|ToggleAimMode
  (Variables|Default|SetbAimMode (not (Variables|Default|GetbAimMode))))

(event Custom|ToggleTick
  (Actor|Tick|SetActorTickEnabled (not (Class|Actor|IsActorTickEnabled))))

(event Custom|SetAutomaticCalibration
  (bind _returnvalue (Class|JoyShockLibrary|JslGetAutoCalibrationStatus))
  (bind _returnvalue_2 (not (.autocalibrationenabled _returnvalue)))
  (Class|JoyShockLibrary|JslSetAutomaticCalibration 0 _returnvalue_2)
  (Development|PrintString (Utilities|String|ToString(Boolean) _returnvalue_2) true false))

(event Custom|StartContinuousCalibration
  (Class|JoyShockLibrary|JslStartContinuousCalibration))

(event Custom|PauseContinuousCalibration
  (Class|JoyShockLibrary|JslPauseContinuousCalibration))

(event Custom|LocalSpace
  (Class|JoyShockLibrary|JslSetGyroSpace))

(event Custom|PlayerSpace
  (Class|JoyShockLibrary|JslSetGyroSpace 0 2))

(event Custom|WorldSpace
  (Class|JoyShockLibrary|JslSetGyroSpace 0 1))

(event EventBeginPlay
  (CallFunction|ConnectDevices)
  (CallFunction|StartContinuousCalibration)
  (Actor|Tick|SetActorTickEnabled true))

(event Collision|EventActorBeginOverlap
  (params (OtherActor :type Actor%20Object%20Reference)))

(event EventTick
  (params (DeltaSeconds :type Float%20%28single-precision%29))
  (bind _returnvalue (Class|JoyShockLibrary|JslGetMotionState))
  (Utilities|FlowControl|Sequence
    (:then_0
      (if (Variables|Default|GetbRotationMode)
        (Transformation|SetActorRotation (Class|KismetMathLibrary|QuatRotator (Utilities|Struct|MakeQuat (* (.quatz _returnvalue) -1.0) (* (.quatx _returnvalue) 1.0) (* (.quaty _returnvalue) -1.0) (.quatw _returnvalue))))))
    (:then_1
      (if (Variables|Default|GetbAimMode)
        (bind (_gyrox _gyroy _gyroz) (Class|JoyShockLibrary|JslGetandFlushAccumulatedGyro))
        (Development|PrintText (Utilities|Text|ToText(String) (Utilities|String|Append "X: " (Utilities|String|ToString(Float) _gyrox) " 
Y: " (Utilities|String|ToString(Float) _gyroy) " 
Z: " (Utilities|String|ToString(Float) _gyroz))) true false "(R=0.000000,G=0.660000,B=1.000000,A=1.000000)" 0.0)
        (Transformation|AddActorWorldOffset (* (Math|Vector|MakeVector 0.0 (* _gyroy -1.0) _gyrox) 1.0))))))

(fn ConstructionScript)